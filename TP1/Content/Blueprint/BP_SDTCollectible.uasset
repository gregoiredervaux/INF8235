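; BP_SDTCollectible is a collectible that reacts with light and sound when a BP_SDTAICharacter overlaps it.
; On begin play it moves its point light to the actor's location, tints it green and assigns a music sound.
; An overlap briefly flashes the light and plays the sound, then a delay-based cooldown flag blocks retriggering for several seconds.
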(event Collision|EventActorBeginOverlap
  (params (OtherActor :type Actor%20Object%20Reference))
  (Utilities|Casting|CastToBP_SDTAICharacter OtherActor)
  (if (not (Variables|Default|GetIsOnCoolDown))
    (Variables|Default|SetIsOnCoolDown true)
    (Rendering|Components|Light|SetIntensity (Variables|Default|GetPointLight) 1e+04)
    (Audio|Components|Audio|Play (Variables|Default|GetSon) 0.0)
    (Utilities|FlowControl|Delay 0.8)
    (Audio|Components|Audio|Stop (Variables|Default|GetSon))
    (Rendering|Components|Light|SetIntensity (Variables|Default|GetPointLight) 0.0)
    (Utilities|FlowControl|Delay 9.0)
    (Variables|Default|SetIsOnCoolDown false)))

(event EventBeginPlay
  (Variables|Default|SetIsOnCoolDown false)
  (Transformation|SetWorldLocation (Variables|Default|GetPointLight) (Transformation|GetActorLocation) false false)
  (Rendering|Components|Light|SetLightColor (Variables|Default|GetPointLight) "(R=0.019557,G=0.630208,B=0.028936,A=1.000000)" true)
  (Audio|Components|Audio|SetSound (Variables|Default|GetSon) "/Game/StarterContent/Audio/Starter_Music01.Starter_Music01"))

(fn ConstructionScript)