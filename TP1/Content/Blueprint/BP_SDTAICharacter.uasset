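; BP_SDTAICharacter is an AI character Blueprint that tallies its own collectible pickups and deaths.
; Both counters reset to zero on BeginPlay.
; Actor overlaps increment NbrCollects for a BP_SDTCollectible that is not on cooldown, or NbrDeaths for a BP_DeathFloor.
; The graph only counts these events, with no respawn, collectible or movement logic.
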(event EventTick
  (params (DeltaSeconds :type Float%20%28single-precision%29)))

(event Collision|EventActorBeginOverlap
  (params (OtherActor :type Actor%20Object%20Reference))
  (bind _asbp_sdtcollectible (Utilities|Casting|CastToBP_SDTCollectible OtherActor)
    (:then
      (if (not (Variables|/Game/Blueprint/BP_SDTCollectible.BP_SDTCollectible_C|GetIsOnCoolDown _asbp_sdtcollectible))
        (Variables|Default|SetnbrCollects (+ (Variables|Default|GetnbrCollects) 1))))
    (:CastFailed
      (Utilities|Casting|CastToBP_DeathFloor OtherActor)
      (Variables|Default|SetnbrDeaths (+ (Variables|Default|GetnbrDeaths) 1)))))

(event EventBeginPlay
  (Variables|Default|SetnbrCollects 0)
  (Variables|Default|SetnbrDeaths 0))

(fn ConstructionScript)